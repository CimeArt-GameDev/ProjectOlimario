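; BP_Press is a level hazard press that repeatedly slams up and down from BeginPlay until its Action event stops the loop.
; A Movement timeline drives the press mesh's Z position and re-triggers Crush on a timer after a configurable delay.
; Timeline event tracks toggle a Crushing window during which box overlaps should deal damage, currently only a debug print placeholder.
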(event OnComponentBeginOverlap(Box)
  (params (OverlappedComponent :type Primitive%20Component%20Object%20Reference) (OtherActor :type Actor%20Object%20Reference) (OtherComp :type Primitive%20Component%20Object%20Reference) (OtherBodyIndex :type Integer) (bFromSweep :type Boolean) (SweepResult :type Hit%20Result%20Structure%20%28by%20ref%29))
  ;[0.03137 0.01961 1] Damage Robot/Player
  (if (Variables|Default|GetCrushing)
    (Development|PrintString "Denis les dégats !!!!" true true "(R=1.000000,G=0.000000,B=0.000000,A=1.000000)" 1e+06)))

(event Custom|Crush
  ;[0 1 0.2431] Crush
  (bind _z_pos (Timeline|Movement PlayFromStart)
    (:Update
      (Transformation|SetRelativeLocation (Variables|Default|GetPress) (Math|Vector|MakeVector 0.0 0.0 _z_pos) false false))
    (:Finished
      ;[0 0.25 0.06078] Loop
      (if (Variables|Default|Getcontinue)
        (Utilities|Time|SetTimerbyEvent (delegate Custom|Crush) (Variables|Default|Getdelaybetweencrushes))))
    (:Start%20crush
      (Variables|Default|SetCrushing true))
    (:Stop%20cruch
      (Variables|Default|SetCrushing false))))

(event EventAction
  ;[1 0 0] Stop
  (Variables|Default|Setcontinue false))

(event EventBeginPlay
  ;[1 0.8627 0] Start
  (CallFunction|Crush))

(fn ConstructionScript)