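; BP_Button_control is a controller that fires linked outputs once all of its linked inputs are pressed, acting as an AND gate for buttons.
; Its Action interface event sets Completed to true, then clears it if any element of the Input array is not Pressed.
; When Completed holds, it calls ActionMessage on every element of the Output array.
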(event EventAction
  ;[1 0 0] Interface call
  ;[0 1 0.2431] Test if completed
  (Variables|Default|SetCompleted true)
  (for _array_element (Variables|Default|GetInput)
    (if (not (Variables|/Game/Core/Level_design/Button/BP_Button.BP_Button_C|GetPressed _array_element))
      (Variables|Default|SetCompleted false)))
  ;[0.03218 0.02061 1] Output
  (if (Variables|Default|GetCompleted)
    (for _array_element_2 (Variables|Default|GetOutput)
      (Class|BPIPuzzles|Action(Message) _array_element_2))))

(fn ConstructionScript)