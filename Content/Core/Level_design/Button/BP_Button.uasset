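; BP_Button is an interactable level button that triggers the actors listed in its Output array.
; On BeginPlay it adds itself to the Input array of any Output entry that is a BP_Button_control.
; The Interact interface event sets a Pressed flag and sends ActionMessage to every Output, ignoring further interactions while that flag stays set.
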(event EventInteract
  (params (Actor :type Actor%20Object%20Reference))
  ;[1 0 0] Interface call
  ;[0 1 0.2431] Test if already pressed
  (if (not (Variables|Default|GetPressed))
    (Variables|Default|SetPressed true)
    ;[0.03137 0.01961 1] Output
    (for _array_element (Variables|Default|GetOutput)
      (Class|BPIPuzzles|Action(Message) _array_element))))

(event EventBeginPlay
  ;[1 0.8627 0] Setup
  (for _array_element (Variables|Default|GetOutput)
    (bind _asbp_button_control (Utilities|Casting|CastToBP_Button_control _array_element))
    (Utilities|Array|Add (Variables|/Game/Core/Level_design/Button/BP_Button_control.BP_Button_control_C|GetInput _asbp_button_control) self)))

(fn ConstructionScript)