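; BP_ConveyorBelt is a puzzle conveyor belt that animates static mesh segments along a spline.
; The construction script spawns a scaled mesh component at spline point indices and stores them in an array.
; Each tick advances every segment by a fixed input-key step from its closest spline key, wrapping to the start past the point count.
; Movement is frame-rate dependent and only sets location, not rotation.
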(event Collision|EventActorBeginOverlap
  (params (OtherActor :type Actor%20Object%20Reference)))

(event EventTick
  (params (DeltaSeconds :type Float%20%28single-precision%29))
  (for _array_element (Variables|Default|GetNewVar_1)
    (Transformation|SetWorldLocation _array_element (Class|SplineComponent|GetLocationatSplineInputKey (Variables|Default|GetSpline) (select (> (+ (Class|SplineComponent|FindInputKeyClosesttoWorldLocation (Variables|Default|GetSpline) (Transformation|GetWorldLocation _array_element)) 0.02) (Math|Conversions|ToFloat(Integer) (Spline|GetNumberOfSplinePoints (Variables|Default|GetSpline)))) 0.0 (+ (Class|SplineComponent|FindInputKeyClosesttoWorldLocation (Variables|Default|GetSpline) (Transformation|GetWorldLocation _array_element)) 0.02)) "World") false false)))

(fn ConstructionScript
  (Utilities|Array|Clear (Variables|Default|GetNewVar_1))
  (for _index (range 0 (Spline|GetNumberOfSplinePoints (Variables|Default|GetSpline)))
    (bind _returnvalue (AddComponent|AddStaticMeshComponent false (Math|Transform|MakeTransform "0, 0, 0" "0, 0, 0" "0.200000,0.500000,0.100000")))
    (Transformation|SetWorldLocation _returnvalue (Spline|GetLocationatSplinePoint (Variables|Default|GetSpline) _index "World") false false)
    (Utilities|Array|Add (Variables|Default|GetNewVar_1) _returnvalue)))