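; BP_Laser is a puzzle laser actor that draws a colored Niagara beam forward from its Sphere component.
; Every tick it line traces on the Visibility channel up to Distance, then sets the beam's end to the hit location, or to full range on a miss.
; It also reapplies LaserColor each tick and only handles the visual, with no reaction on whatever the beam hits.
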(event EventTick
  (params (DeltaSeconds :type Float%20%28single-precision%29))
  (bind _sphere (Variables|Default|GetSphere))
  (bind _distance (Variables|Default|GetDistance))
  (bind _returnvalue (Transformation|GetWorldLocation _sphere))
  (bind _returnvalue_2 (Math|Vector|GetForwardVector _sphere))
  (bind _returnvalue_3 (* _returnvalue_2 _distance))
  (bind _returnvalue_4 (+ _returnvalue _returnvalue_3))
  (Effects|Components|ParticleSystem|SetColorParameter (Variables|Default|GetNiagara_Laser) "Color" (Variables|Default|GetLaserColor))
  (bind (_outhit _returnvalue_5) (Collision|LineTraceByChannel _returnvalue _returnvalue_4 "TraceTypeQuery1" false 0 "None"))
  (Effects|Components|ParticleSystem|SetVectorParameter (Variables|Default|GetNiagara_Laser) "LaserEnd" (select _returnvalue_5 (.Location (Collision|BreakHitResult _outhit)) _returnvalue_4)))

(fn ConstructionScript)