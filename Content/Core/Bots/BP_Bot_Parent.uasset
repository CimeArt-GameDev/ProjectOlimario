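; Parent Blueprint for AI bots that register with the player, ragdoll when sent to work, then get up and work for a timed duration.
; WorkStart enables hips-down physics while line traces keep the capsule under the ragdoll.
; Once the mesh settles, a pose snapshot and timeline realign it during the ABP_Bot get-up.
; BeginWork is an empty hook, and WorkEnd resets the Blackboard state.
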(event Custom|GetUp
  (Default|SaveSnapShot (Variables|Default|GetanimBPBot))
  (Pawn|Components|CharacterMovement|SetMovementMode (Variables|Character|GetCharacterMovement) "MOVE_Walking" 0)
  (Variables|gettingUp|SetbThrown false)
  (Class|SkeletalMeshComponent|SetAllBodiesBelowSimulatePhysics (Variables|Character|GetMesh) (Utilities|Name|MakeLiteralName "robo_Hips") false true)
  (Collision|SetCollisionEnabled (Variables|Collision|GetCapsuleComponent) "QueryAndPhysics")
  (Transformation|AttachComponentToComponent (Variables|Character|GetMesh) (Variables|Collision|GetCapsuleComponent) "None" "KeepWorld" "KeepWorld" "KeepRelative" false)
  (Utilities|FlowControl|Delay 0.1)
  (Utilities|FlowControl|Sequence
    (:then_0
      (Variables|gettingUp|SettempMeshWorldRotationZ (.yaw (Transformation|GetWorldRotation (Variables|Character|GetMesh))))
      (Variables|gettingUp|SettempMeshDirectionBetweenSocketsZ (.yaw (Math|Rotator|MakeRotfromX (Class|KismetAnimationLibrary|DirectionBetweenSockets (Variables|Character|GetMesh) "robo_Neck1" "robo_Hips"))))
      (bind _alpha (Timeline|timelineRotationLocationWhileGettingUp PlayFromStart)
        (:Update
          (Transformation|SetRelativeLocation (Variables|Character|GetMesh) (Math|Vector|MakeVector 0.0 0.0 (Math|Float|Lerp -5e+01 -93.0 _alpha)) false false)
          (Transformation|SetWorldRotation (Variables|Character|GetMesh) (Math|Rotator|MakeRotator 0.0 0.0 (Math|Float|Lerp (Variables|gettingUp|GettempMeshWorldRotationZ) (Variables|gettingUp|GettempMeshDirectionBetweenSocketsZ) _alpha)) false false))))
    (:then_1
      (bind _animduration (Default|GettUp (Variables|Default|GetanimBPBot)))
      (bind _returnvalue (Utilities|Time|SetTimerbyEvent (delegate Custom|isUp) _animduration)))))

(event Custom|WorkEnd
  (Development|PrintString "Job Done !")
  (AI|Components|Blackboard|SetValueasEnum (Variables|/Script/AIModule.AIController|GetBlackboard (AI|GetAIController self)) (Variables|AI|GetbotStateKeyName))
  (Transformation|SetRelativeRotation (Variables|Character|GetMesh) "0,-90.000000, 0" false false)
  (Utilities|Time|ClearandInvalidateTimerbyHandle (Variables|work|GetworkTimer)))

(event Custom|WorkStart
  (Variables|Default|SetthrowDirection (Transformation|GetActorForwardVector (Variables|Default|GetrefPlayer)))
  (Pawn|Components|CharacterMovement|DisableMovement (Variables|Character|GetCharacterMovement))
  (Class|SkeletalMeshComponent|SetAllBodiesBelowSimulatePhysics (Variables|Character|GetMesh) (Utilities|Name|MakeLiteralName "robo_Hips") true true)
  (Class|SkeletalMeshComponent|SetAllBodiesBelowPhysicsBlendWeight (Variables|Character|GetMesh) (Utilities|Name|MakeLiteralName "robo_Hips") 1.0 false true)
  (Collision|SetCollisionEnabled (Variables|Character|GetMesh) "QueryAndPhysics")
  (Collision|SetCollisionEnabled (Variables|Collision|GetCapsuleComponent) "NoCollision")
  (Variables|gettingUp|SetbThrown true)
  (Utilities|Time|SetTimerbyFunctionName 0 "StartGetUp" 2.0))

(event Custom|isUp
  (Utilities|Time|ClearandInvalidateTimerbyHandle (stale Custom|GetUp _returnvalue))
  (Transformation|SetRelativeRotation (Variables|Character|GetMesh) "0,-90.000000, 0" false false)
  (bind _returnvalue (Utilities|Time|SetTimerbyEvent (delegate Custom|WorkEnd) (Variables|work|GetworkDuration)))
  (Variables|work|SetworkTimer _returnvalue)
  (CallFunction|BeginWork))

(event Custom|beginWork)

(event EventBeginPlay
  (AI|Components|Blackboard|SetValueasObject (Variables|/Script/AIModule.AIController|GetBlackboard (AI|GetAIController self)) (Variables|AI|GetplayerKeyName) (Game|GetPlayerCharacter 0))
  (bind _asabp_bot (Utilities|Casting|CastToABP_Bot (Components|SkeletalMesh|GetAnimInstance (Variables|Character|GetMesh))))
  (Variables|Default|SetanimBPBot _asabp_bot)
  (bind _astemp_test_character_denis (Utilities|Casting|CastToTemp_TestCharacter_Denis (Game|GetPlayerCharacter 0)))
  (Variables|Default|SetrefPlayer _astemp_test_character_denis)
  (bind _astemp_test_character_denis_2 (Utilities|Casting|CastToTemp_TestCharacter_Denis (Game|GetPlayerCharacter 0)))
  (Utilities|Array|Add (Variables|/Game/Core/Bots/Temp_TestCharacter_Denis.Temp_TestCharacter_Denis_C|GetbotsArray _astemp_test_character_denis_2) self))

(event EventTick
  (params (DeltaSeconds :type Float%20%28single-precision%29))
  (CallFunction|GetUpCheck))

(fn ConstructionScript)

(fn GetUpCheck
  (bind _mesh (Variables|Character|GetMesh))
  (bind _returnvalue (Transformation|GetComponentVelocity _mesh))
  (bind _returnvalue_2 (Math|Vector|VectorLength _returnvalue))
  (bind _returnvalue_3 (Math|Float|Truncate _returnvalue_2))
  (if (Variables|gettingUp|GetbGetUpCheck)
    (if (and (> _returnvalue_3 -10) (< _returnvalue_3 10))
      (CallFunction|MoveCapsule)
      (CallFunction|GetUp)
      (Variables|gettingUp|SetbGetUpCheck false))
    (else
      (CallFunction|MoveCapsule))))

(fn MoveCapsule
  (bind _mesh (Variables|Character|GetMesh))
  (bind _returnvalue (Transformation|GetSocketLocation _mesh "robo_Hips"))
  (if (Variables|gettingUp|GetbThrown)
    (bind (_outhit _returnvalue_2) (Collision|LineTraceByChannel _returnvalue (+ _returnvalue (* (Transformation|GetActorUpVector) -2e+02)) "TraceTypeQuery1" false 0 "None"))
    (if _returnvalue_2
      (Variables|gettingUp|SetcapsuleLocation (+ (.impactpoint _outhit) (Math|Vector|MakeVector 0.0 0.0 (+ (Components|Capsule|GetScaledCapsuleHalfHeight (Variables|Collision|GetCapsuleComponent)) 3.0))))
      (Transformation|SetWorldLocation (Variables|Collision|GetCapsuleComponent) (Variables|gettingUp|GetcapsuleLocation) false false)
      (Transformation|SetWorldRotation (Variables|Collision|GetCapsuleComponent) (Math|Rotator|MakeRotator 0.0 0.0 (.yaw (Math|Rotator|MakeRotfromX (Class|KismetAnimationLibrary|DirectionBetweenSockets (Variables|Character|GetMesh) "robo_Neck" "robo_Hips")))) false false))))

(fn StartGetUp
  (Variables|gettingUp|SetbGetUpCheck true))