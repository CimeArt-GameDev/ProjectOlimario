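; Bot Blueprint named as a slowing variant, built around a Sphere trigger that reacts to the Temp_TestCharacter_Denis test character.
; Beginning an overlap with that character drops CustomTimeDilation to a fifth of normal speed.
; The end-overlap handler only casts and never restores the speed.
; Blackboard bot-state checks meant to gate both handlers are disconnected, and BeginWork is empty, so the behavior looks unfinished.
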(event OnComponentBeginOverlap(Sphere)
  (params (OverlappedComponent :type Primitive%20Component%20Object%20Reference) (OtherActor :type Actor%20Object%20Reference) (OtherComp :type Primitive%20Component%20Object%20Reference) (OtherBodyIndex :type Integer) (bFromSweep :type Boolean) (SweepResult :type Hit%20Result%20Structure%20%28by%20ref%29))
  (Utilities|Casting|CastToTemp_TestCharacter_Denis OtherActor)
  (Variables|Default|SetCustomTimeDilation 0.2))

(event OnComponentEndOverlap(Sphere)
  (params (OverlappedComponent :type Primitive%20Component%20Object%20Reference) (OtherActor :type Actor%20Object%20Reference) (OtherComp :type Primitive%20Component%20Object%20Reference) (OtherBodyIndex :type Integer))
  (Utilities|Casting|CastToTemp_TestCharacter_Denis OtherActor))

(event EventBeginPlay
  (|CallParentFunction) ; This node is disabled and will not be called.\nDrag off pins to build functionality.
)

(event Collision|EventActorBeginOverlap
  (params (OtherActor :type Actor%20Object%20Reference)))

(event EventTick
  (params (DeltaSeconds :type Float%20%28single-precision%29))
  (|CallParentFunction DeltaSeconds) ; This node is disabled and will not be called.\nDrag off pins to build functionality.
)

(event EventBeginWork)

(fn ConstructionScript
  (|CallParentFunction))