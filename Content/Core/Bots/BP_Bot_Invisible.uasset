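; Bot subclass that cloaks third-person characters inside its sphere while traveling in the direction it was thrown.
; On BeginWork it line-traces along ThrowDirection and AI-moves to the hit point, or to a distant point if nothing is hit.
; While the blackboard bot state has one specific value, sphere overlaps toggle the character's IsInvisible flag and swap its mesh between noise and body materials.
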(event OnComponentBeginOverlap(Sphere)
  (params (OverlappedComponent :type Primitive%20Component%20Object%20Reference) (OtherActor :type Actor%20Object%20Reference) (OtherComp :type Primitive%20Component%20Object%20Reference) (OtherBodyIndex :type Integer) (bFromSweep :type Boolean) (SweepResult :type Hit%20Result%20Structure%20%28by%20ref%29))
  (if (== (Class|BlackboardComponent|GetValueasEnum (Variables|/Script/AIModule.AIController|GetBlackboard (AI|GetAIController self)) (Variables|Default|GetbotStateKeyName)) 3)
    (bind _asthird_person_character (Utilities|Casting|CastToThirdPersonCharacter OtherActor))
    (Variables|/Game/Core/Character/ThirdPersonCharacter.ThirdPersonCharacter_C|SetisInvisible _asthird_person_character true)
    (Rendering|Material|SetMaterial (Variables|/Script/Engine.Character|GetMesh _asthird_person_character) 0 "/Game/Misc/Materials/M_Noise.M_Noise")))

(event OnComponentEndOverlap(Sphere)
  (params (OverlappedComponent :type Primitive%20Component%20Object%20Reference) (OtherActor :type Actor%20Object%20Reference) (OtherComp :type Primitive%20Component%20Object%20Reference) (OtherBodyIndex :type Integer))
  (if (== (Class|BlackboardComponent|GetValueasEnum (Variables|/Script/AIModule.AIController|GetBlackboard (AI|GetAIController self)) (Variables|Default|GetbotStateKeyName)) 3)
    (bind _asthird_person_character (Utilities|Casting|CastToThirdPersonCharacter OtherActor))
    (Variables|/Game/Core/Character/ThirdPersonCharacter.ThirdPersonCharacter_C|SetisInvisible _asthird_person_character false)
    (Rendering|Material|SetMaterial (Variables|/Script/Engine.Character|GetMesh _asthird_person_character) 0 "/Game/Characters/Mannequin/Materials/M_Male_Body.M_Male_Body")))

(event EventBeginPlay
  (|CallParentFunction) ; This node is disabled and will not be called.\nDrag off pins to build functionality.
)

(event Collision|EventActorBeginOverlap
  (params (OtherActor :type Actor%20Object%20Reference))
  (|CallParentFunction OtherActor) ; This node is disabled and will not be called.\nDrag off pins to build functionality.
)

(event EventTick
  (params (DeltaSeconds :type Float%20%28single-precision%29))
  (|CallParentFunction DeltaSeconds) ; This node is disabled and will not be called.\nDrag off pins to build functionality.
)

(event EventWorkStart
  (|CallParentFunction)
  (Variables|Default|SetDestination (* (Transformation|GetActorForwardVector (Variables|Default|GetrefPlayer)) 1e+04)))

(event EventBeginWork
  (bind _returnvalue (Transformation|GetActorLocation))
  (bind _throwdirection (Variables|Default|GetthrowDirection))
  (bind _returnvalue_2 (* _throwdirection 1e+05))
  (bind _returnvalue_3 (+ _returnvalue _returnvalue_2))
  (|CallParentFunction)
  (bind (_outhit _returnvalue_4) (Collision|LineTraceByChannel (Transformation|GetActorLocation) _returnvalue_3 "TraceTypeQuery1" false 0 "None"))
  (if _returnvalue_4
    (AI|AIMoveTo self (.Location (Collision|BreakHitResult _outhit)) 0 5.0 false)
    (else
      (AI|AIMoveTo self _returnvalue_3 0 5.0 false))))

(fn ConstructionScript
  (|CallParentFunction))