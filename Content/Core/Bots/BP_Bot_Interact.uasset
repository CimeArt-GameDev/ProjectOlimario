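; Player-controllable bot character that interacts with puzzle actors and can hand control back to CharaTestLucien with M.
; Axis inputs drive yaw-relative planar movement and camera look, while R fires a short camera line trace that sends InteractMessage to BPI_Puzzles actors.
; Possession creates a crosshair widget, removed on unpossession and also, through a DoOnce, right after the first possession.
; Tick prints the movement mode for debugging.
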(event EventBeginPlay
  (|CallParentFunction))

(event Collision|EventActorBeginOverlap
  (params (OtherActor :type Actor%20Object%20Reference))
  (|CallParentFunction OtherActor) ; This node is disabled and will not be called.\nDrag off pins to build functionality.
)

(event EventPossessed
  (params (NewController :type Controller%20Object%20Reference))
  ;[1 1 1] HUD
  (bind _returnvalue (UserInterface|CreateWidget "/Game/Core/UI/Blueprints/WBP_Crosshair.WBP_Crosshair_C"))
  (UserInterface|Viewport|AddtoViewport _returnvalue 0)
  (Utilities|FlowControl|DoOnce false
    (:Completed
      (Widget|RemovefromParent _returnvalue))))

(event EventUnpossessed
  (params (OldController :type Controller%20Object%20Reference))
  ;[1 1 1] HUD
  (Widget|RemovefromParent (stale EventPossessed _returnvalue)))

(event EventTick
  (params (DeltaSeconds :type Float%20%28single-precision%29))
  (Development|PrintString (Utilities|String|EnumtoString (Variables|/Script/Engine.CharacterMovementComponent|GetMovementMode (Variables|Character|GetCharacterMovement))) true true "(R=0.000000,G=0.660000,B=1.000000,A=1.000000)" 0.0))

(event Input|AxisEvents|InputAxisLookUp
  (params (AxisValue :type Float%20%28single-precision%29))
  ;[1 1 1] Movement
  (Pawn|Input|AddControllerPitchInput AxisValue))

(event Input|AxisEvents|InputAxisTurn
  (params (AxisValue :type Float%20%28single-precision%29))
  ;[1 1 1] Movement
  (Pawn|Input|AddControllerYawInput AxisValue))

(event Input|AxisEvents|InputAxisMoveForward
  (params (AxisValue :type Float%20%28single-precision%29))
  ;[1 1 1] Movement
  (Pawn|Input|AddMovementInput (Math|Vector|GetForwardVector (Math|Rotator|MakeRotator 0.0 0.0 (.Yaw (Math|Rotator|BreakRotator (Pawn|GetControlRotation :!class /Script/Engine.Pawn))))) AxisValue false))

(event Input|AxisEvents|InputAxisMoveRight
  (params (AxisValue :type Float%20%28single-precision%29))
  ;[1 1 1] Movement
  (Pawn|Input|AddMovementInput (Math|Vector|GetRightVector (Math|Rotator|MakeRotator 0.0 0.0 (.Yaw (Math|Rotator|BreakRotator (Pawn|GetControlRotation :!class /Script/Engine.Pawn))))) AxisValue false))

(event Input|KeyboardEvents|R
  (params (Key :type Key%20Structure :default "None"))
  (bind _camera (Variables|Actor|GetCamera))
  (bind _returnvalue (Transformation|GetWorldLocation _camera))
  ;[1 1 1] Interact
  (:Pressed
    (bind (_outhit _returnvalue_2) (Collision|LineTraceByChannel _returnvalue (+ _returnvalue (* (Math|Vector|GetForwardVector _camera) 2e+02)) "TraceTypeQuery1" false 0 "ForDuration"))
    (if _returnvalue_2
      (if (Utilities|DoesObjectImplementInterface (.HitActor (Collision|BreakHitResult _outhit)) "/Game/Core/Level_design/BPI_Puzzles.BPI_Puzzles_C")
        (Class|BPIPuzzles|Interact(Message) (.HitActor (Collision|BreakHitResult _outhit)) self)))))

(event Input|KeyboardEvents|M
  (params (Key :type Key%20Structure :default "None"))
  ;[1 1 1] PossessPlayer
  (:Pressed
    (bind _outactors (Actor|GetAllActorsOfClass "/Game/Core/Character/CharaTestLucien.CharaTestLucien_C"))
    (for _array_element _outactors
      (Pawn|Possess (Game|GetPlayerController 0) _array_element))))

(fn ConstructionScript
  (|CallParentFunction))